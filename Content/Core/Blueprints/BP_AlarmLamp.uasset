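; BP_AlarmLamp is the bathyscaphe's damage warning lamp, signalling cracks with light and sound.
; Every tick it reads CracksCount from BP_PalyerController, showing the rect light and raising the alarm's volume multiplier while cracks exist, otherwise hiding and silencing them.
; It also implements interaction functions that supply its info text and interact type, with grab interaction returning a zero vector.
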(event `self.ReceiveTick`
  (params (DeltaSeconds :type "Float (single-precision)"))
  (bind _rectlight (`self.RectLight`))
  (bind _asbp_palyer_controller (cast `/Game/Core/Blueprints/BP_PalyerController` (`GameplayStatics.GetPlayerController` 0)))
  (if (> (`/Game/Core/Blueprints/BP_PalyerController.CracksCount` _asbp_palyer_controller) 0)
    (`SceneComponent.SetVisibility` _rectlight true false)
    (`AudioComponent.SetVolumeMultiplier` (`self.SC_Alarm`) 2.0)
    (else
      (`SceneComponent.SetVisibility` _rectlight false false)
      (`AudioComponent.SetVolumeMultiplier` (`self.SC_Alarm`) 0.0))))

(fn `GetInfoText`
  (returns (Info :type Text))
  (return "Bathyscaphe damage warning lamp"))

(fn `GetTypeInteract`
  (returns (Type :type "/Game/Core/Blueprints/E_TypeInteract Enum"))
  (return "NewEnumerator2"))

(fn `Grab Interact`
  (params (`Player aim movement` :type "Vector2D Structure") (Interacting :type Boolean))
  (returns (`Player focus target` :type "Vector Structure"))
  (return (0.0 0.0 0.0)))

(fn `UserConstructionScript`)