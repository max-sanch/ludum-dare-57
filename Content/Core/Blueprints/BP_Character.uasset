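; First-person player character Blueprint that handles mouse look, object interaction and audio feedback for CO2 and pressure levels.
; Left click traces from the camera for BPI_Interact actors, then either pushes them or starts a hold-to-grab.
; While grabbing, look input feeds the actor instead of the camera, which eases toward the actor's returned target.
; Tick scales breathing and Tnturner sound volumes from player controller values above thresholds.
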(event `InputAxis|Turn` :overrideparent false
  (params (AxisValue :type "Float (single-precision)"))
  ;[1 1 1] Look
  (if (not (`self.Interacting`))
    (`self.AddControllerYawInput` AxisValue)))

(event `Key|LeftMouseButton`
  (params (Key :type "Key Structure"))
  ;[1 1 1] Interact Button
  (:`Pressed`
    (`self.Sight Line Tracing `)
    (`/Engine/EditorBlueprintResources/StandardMacros.IsValid` (`self.InteractableActor`)
      (:`Is Valid`
        (bind _type (message `/Game/Core/Blueprints/BPI_Interact.GetTypeInteract` (`self.InteractableActor`)))
        (switch `/Game/Core/Blueprints/E_TypeInteract` _type
          (:`NewEnumerator0`
            (set `self.Interacting` true))
          (:`NewEnumerator1`
            (message `/Game/Core/Blueprints/BPI_Interact.Push Interact` (`self.InteractableActor`) self))))))
  (:`Released`
    (set `self.Interacting` false)))

(event `InputAxis|LookUp` :overrideparent false
  (params (AxisValue :type "Float (single-precision)"))
  ;[1 1 1] Look
  (if (not (`self.Interacting`))
    (`self.AddControllerPitchInput` AxisValue)))

(event `self.ReceiveTick`
  (params (DeltaSeconds :type "Float (single-precision)"))
  (set `self.Delta Seconds` DeltaSeconds)
  (`|ExecutionSequence`
    (:`then_0`
      ;[1 1 1] Interact
      (if (`self.Interacting`)
        (bind _player_focus_target (message `/Game/Core/Blueprints/BPI_Interact.Grab Interact` (`self.InteractableActor`) (`KismetMathLibrary.MakeVector2D` (`self.GetInputAxisValue`) (`self.GetInputAxisValue`)) true))
        (`Controller.SetControlRotation` (`GameplayStatics.GetPlayerController` 0) (`KismetMathLibrary.RInterpTo` (`Controller.GetControlRotation` (`GameplayStatics.GetPlayerController` 0)) (`KismetMathLibrary.FindLookAtRotation` (`SceneComponent.K2_GetComponentLocation` (`self.Camera`)) _player_focus_target) (`self.Delta seconds`) 15.0))
        (goto _label :!via `Reset`)
        (else
          (`/Engine/EditorBlueprintResources/StandardMacros.DoOnce` true :!label _label
            (:`Completed`
              (message `/Game/Core/Blueprints/BPI_Interact.Grab Interact` (`self.InteractableActor`) (0.0 0.0) false))))))
    (:`then_1`
      (bind _asbp_palyer_controller (cast `/Game/Core/Blueprints/BP_PalyerController` (`GameplayStatics.GetPlayerController` 0)))
      (`|ExecutionSequence`
        (:`then_0`
          (bind _carbondioxidevalue (`/Game/Core/Blueprints/BP_PalyerController.CarbonDioxideValue` _asbp_palyer_controller))
          ;[1 1 1] Breath
          (if (> _carbondioxidevalue 30.0)
            (`AudioComponent.SetVolumeMultiplier` (`self.SC_Breath`) (* (/ (- _carbondioxidevalue 29.0) 30.0) 2.0))
            (else
              (`AudioComponent.SetVolumeMultiplier` (`self.SC_Breath`) 0.0))))
        (:`then_1`
          (bind _pressurevalue (`/Game/Core/Blueprints/BP_PalyerController.PressureValue` _asbp_palyer_controller))
          ;[1 1 1] Tnturner
          (if (> _pressurevalue 2.0)
            (`AudioComponent.SetVolumeMultiplier` (`self.SC_Tnturner`) (- _pressurevalue 1.98))
            (else
              (`AudioComponent.SetVolumeMultiplier` (`self.SC_Tnturner`) 0.0))))))))

(fn `Sight Line Tracing `
  (locals (InteractDistance :type "Float (double-precision)" :default 5000.0))
  (bind _camera (`self.Camera`))
  (bind _returnvalue (`SceneComponent.K2_GetComponentLocation` _camera))
  (bind _outhit (`KismetSystemLibrary.LineTraceSingle` _returnvalue (+ _returnvalue (* (`SceneComponent.GetForwardVector` _camera) (`local.InteractDistance`))) "TraceTypeQuery1"))
  (bind (_bblockinghit _binitialoverlap _time _distance _location _impactpoint _normal _impactnormal _physmat _hitactor) (`GameplayStatics.BreakHitResult` _outhit))
  (if _bblockinghit
    (if (`KismetSystemLibrary.DoesImplementInterface` _hitactor "/Game/Core/Blueprints/BPI_Interact.BPI_Interact_C")
      (set `self.InteractableActor` _hitactor)
      (else
        (set `self.InteractableActor` null :!label _label)))
    (else
      (goto _label))))

(fn `UserConstructionScript`)