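; BP_CrackGlass is an interactable cracked glass object that the player can patch with tape.
; It answers interaction calls with a fixed interact type, and its grab interaction only returns a zero vector.
; A push interaction, when the glass is not hidden and not yet repaired, sets the repaired flag and swaps the Cube's material to tape, so the repair happens only once.
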(fn `GetTypeInteract`
  (returns (Type :type "/Game/Core/Blueprints/E_TypeInteract Enum"))
  (return "NewEnumerator1"))

(fn `Grab Interact`
  (params (`Player aim movement` :type "Vector2D Structure") (Interacting :type Boolean))
  (returns (`Player focus target` :type "Vector Structure"))
  (return (0.0 0.0 0.0)))

(fn `Push Interact`
  (params (Character :type "/Game/Core/Blueprints/BP_Character Object Reference"))
  (if (`self.IsHidden`)
    _
    (elif (not (`self.IsRepaired`))
      (set `self.IsRepaired` true)
      (`PrimitiveComponent.SetMaterial` (`self.Cube`) 0 "/Game/Core/Materials/M_Tape.M_Tape")
      (return))))

(fn `UserConstructionScript`)