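; BP_Helm is an interactable steering wheel that the player drags to change the bathyscaphe's inclination.
; Grab interaction turns horizontal aim movement past a threshold into small, clamped yaw steps on the helm mesh and returns its focus socket location.
; Tick eases the wheel back toward center, converting its yaw into the player controller's SlantSpeed and scaling the slant engine sound's volume with that speed's magnitude.
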(event `self.ReceiveTick`
  (params (DeltaSeconds :type "Float (single-precision)"))
  (bind (_relativerotation_roll _relativerotation_pitch _relativerotation_yaw) (`KismetMathLibrary.BreakRotator` (`SceneComponent.RelativeRotation` (`self.SM_Helm`))))
  (bind (_relativerotation_roll_2 _relativerotation_pitch_2 _relativerotation_yaw_2) (`KismetMathLibrary.BreakRotator` (`SceneComponent.RelativeRotation` (`self.SM_Helm`))))
  (`SceneComponent.K2_SetRelativeRotation` (`self.SM_Helm`) (`KismetMathLibrary.MakeRotator` _relativerotation_roll_2 _relativerotation_pitch_2 (`KismetMathLibrary.FInterpTo` _relativerotation_yaw_2 0.0 DeltaSeconds 3.0)) false false)
  (bind _asbp_palyer_controller (cast `/Game/Core/Blueprints/BP_PalyerController` (`GameplayStatics.GetPlayerController` 0)))
  (if (== _relativerotation_yaw 0.0)
    (set `/Game/Core/Blueprints/BP_PalyerController.SlantSpeed` 0.0 _asbp_palyer_controller)
    (`AudioComponent.SetVolumeMultiplier` (`self.SC_SlantEngine`) 0.0)
    (else
      (bind _output_get (set `/Game/Core/Blueprints/BP_PalyerController.SlantSpeed` (/ _relativerotation_yaw 10.0) _asbp_palyer_controller))
      (`AudioComponent.SetVolumeMultiplier` (`self.SC_SlantEngine`) (* (`KismetMathLibrary.Abs` _output_get) 3.0)))))

(event `Move switch`
  (bind (_relativerotation_roll _relativerotation_pitch _relativerotation_yaw) (`KismetMathLibrary.BreakRotator` (`SceneComponent.RelativeRotation` (`self.SM_Helm`))))
  (if (`self.ToRight`)
    (set `self.RotateDiff` -0.2)
    (else
      (set `self.RotateDiff` 0.2)))
  (`SceneComponent.K2_SetRelativeRotation` (`self.SM_Helm`) (`KismetMathLibrary.MakeRotator` _relativerotation_roll _relativerotation_pitch (`KismetMathLibrary.FClamp` (+ _relativerotation_yaw (`self.RotateDiff`)) -30.0 30.0)) false false))

(fn `GetInfoText`
  (returns (Info :type Text))
  (return "Steering wheel for changing the inclination of the bathyscaphe. Hold and drag"))

(fn `GetTypeInteract`
  (returns (Type :type "/Game/Core/Blueprints/E_TypeInteract Enum"))
  (return "NewEnumerator0"))

(fn `Grab Interact`
  (params (`Player aim movement` :type "Vector2D Structure") (Interacting :type Boolean))
  (returns (`Player focus target` :type "Vector Structure"))
  (bind _x (`KismetMathLibrary.BreakVector2D` `Player aim movement`))
  (bind _returnvalue (>= _x 0.5))
  (if (or _returnvalue (<= _x -0.5))
    (set `self.ToRight` _returnvalue)
    (`self.Move switch`))
  (return (`SceneComponent.GetSocketLocation` (`self.SM_Helm`) "Focus target")))

(fn `UserConstructionScript`)