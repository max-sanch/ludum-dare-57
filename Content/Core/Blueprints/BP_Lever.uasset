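; BP_Lever is a grabbable speed control lever that sets the player controller's speed value and drives the main engine sound.
; Grab interaction turns vertical aim movement past a threshold into small, clamped pitch steps on the handle, returning a focus socket location.
; Every tick, the handle's pitch is mapped to the controller's speed, which scales engine volume and pitch, muting it at zero.
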(event `self.ReceiveTick`
  (params (DeltaSeconds :type "Float (single-precision)"))
  (bind (_relativerotation_roll _relativerotation_pitch) (`KismetMathLibrary.BreakRotator` (`SceneComponent.RelativeRotation` (`self.Switch_Handle`))))
  (bind _asbp_palyer_controller (cast `/Game/Core/Blueprints/BP_PalyerController` (`GameplayStatics.GetPlayerController` 0)))
  (bind _output_get (set `/Game/Core/Blueprints/BP_PalyerController.SpeedValue` (`KismetMathLibrary.FClamp` (+ _relativerotation_pitch 30.0) 0.0 60.0) _asbp_palyer_controller))
  (if (== _output_get 0.0)
    (`AudioComponent.SetVolumeMultiplier` (`self.SC_MainEngine`) 0.0)
    (else
      (`AudioComponent.SetVolumeMultiplier` (`self.SC_MainEngine`) (* (/ _output_get 60.0) 3.0))
      (`AudioComponent.SetPitchMultiplier` (`self.SC_MainEngine`) (+ (/ _output_get 120.0) 0.5)))))

(event `Move switch`
  (bind (_relativerotation_roll _relativerotation_pitch _relativerotation_yaw) (`KismetMathLibrary.BreakRotator` (`SceneComponent.RelativeRotation` (`self.Switch_Handle`))))
  (if (`self.ToUp`)
    (set `self.RotateDiff` -0.5)
    (else
      (set `self.RotateDiff` 0.5)))
  (`SceneComponent.K2_SetRelativeRotation` (`self.Switch_Handle`) (`KismetMathLibrary.MakeRotator` _relativerotation_roll (`KismetMathLibrary.FClamp` (+ _relativerotation_pitch (`self.RotateDiff`)) -30.0 30.0) _relativerotation_yaw) false false))

(fn `GetInfoText`
  (returns (Info :type Text))
  (return "The speed control lever. Hold and drag"))

(fn `GetTypeInteract`
  (returns (Type :type "/Game/Core/Blueprints/E_TypeInteract Enum"))
  (return "NewEnumerator0"))

(fn `Grab Interact`
  (params (`Player aim movement` :type "Vector2D Structure") (Interacting :type Boolean))
  (returns (`Player focus target` :type "Vector Structure"))
  (bind (_x _y) (`KismetMathLibrary.BreakVector2D` `Player aim movement`))
  (bind _returnvalue (>= _y 0.5))
  (if (or _returnvalue (<= _y -0.5))
    (set `self.ToUp` _returnvalue)
    (`self.Move switch`))
  (return (`SceneComponent.GetSocketLocation` (`self.Switch_Handle`) "Focus target")))

(fn `Push Interact`
  (params (Character :type "/Game/Core/Blueprints/BP_Character Object Reference"))
  (return))

(fn `UserConstructionScript`)